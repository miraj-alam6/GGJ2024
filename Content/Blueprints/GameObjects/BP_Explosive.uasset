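; Proximity-triggered explosive physics prop that counts down, then damages the player and pushes nearby physics actors.
; Overlapping the proximity volume starts the countdown, during which Tick drives a material Frequency parameter as a warning and keeps a scene component on the simulated mesh.
; A radius volume tracks the player and CustomPhysicsActors, which receive outward force scaled by squared-distance falloff on detonation.
; The mesh then hides and the actor is destroyed after a delay.
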(event `self.ReceiveBeginPlay`
  (`parent.ReceiveBeginPlay`)
  (`PrimitiveComponent.SetCollisionEnabled` (`self.ProximityOverlap`) "NoCollision")
  (`PrimitiveComponent.SetCollisionEnabled` (`self.Explosiion Radius`) "NoCollision")
  (`KismetSystemLibrary.Delay` 0.0)
  (`PrimitiveComponent.SetCollisionEnabled` (`self.ProximityOverlap`) "QueryOnly")
  (`PrimitiveComponent.SetCollisionEnabled` (`self.Explosiion Radius`) "QueryOnly"))

(event `self.ReceiveTick`
  (params (DeltaSeconds :type "Float (single-precision)"))
  (`parent.ReceiveTick` DeltaSeconds)
  (`SceneComponent.K2_SetWorldLocation` (`self.SceneThatFollows`) (`SceneComponent.K2_GetComponentLocation` (`self.StaticMesh`)) false true)
  (`self.AboutToExplodeTick` DeltaSeconds)
  (`self.TryExplode`))

(event `self.ProximityOverlap.OnComponentBeginOverlap`
  (params (OverlappedComponent :type "PrimitiveComponent Object Reference") (OtherActor :type "Actor Object Reference") (OtherComp :type "PrimitiveComponent Object Reference") (OtherBodyIndex :type Integer) (bFromSweep :type Boolean) (SweepResult :type "HitResult Structure (by ref)"))
  (`self.BeginCountdown`))

(event `self.Explosiion Radius.OnComponentBeginOverlap`
  (params (OverlappedComponent :type "PrimitiveComponent Object Reference") (OtherActor :type "Actor Object Reference") (OtherComp :type "PrimitiveComponent Object Reference") (OtherBodyIndex :type Integer) (bFromSweep :type Boolean) (SweepResult :type "HitResult Structure (by ref)"))
  (bind _ascustom_physics_actor (cast `CustomPhysicsActor` OtherActor)
    (:`then`
      (`KismetArrayLibrary.Array_Add` (`self.PhysicsActorsInRadius`) _ascustom_physics_actor))
    (:`CastFailed`
      (bind _asplayer_character (cast `PlayerCharacter` OtherActor))
      (set `self.PlayerInExplosionRadius` _asplayer_character))))

(event `self.Explosiion Radius.OnComponentEndOverlap`
  (params (OverlappedComponent :type "PrimitiveComponent Object Reference") (OtherActor :type "Actor Object Reference") (OtherComp :type "PrimitiveComponent Object Reference") (OtherBodyIndex :type Integer))
  (cast `CustomPhysicsActor` OtherActor
    (:`then`
      (`KismetArrayLibrary.Array_RemoveItem` (`self.PhysicsActorsInRadius`) self))
    (:`CastFailed`
      (cast `PlayerCharacter` OtherActor)
      ;[1 1 1] Clear ref
      (set `self.PlayerInExplosionRadius` null))))

(event `TryExplode`
  (bind _staticmesh (`self.StaticMesh`))
  (if (`self.bExploded`)
    _
    (elif (and (`self.bDoingCountdown`) (<= (`self.ExplosionCountdownLeft`) 1e-06))
      (set `self.bExploded` true)
      (`self.Apply Forces and Damage`)
      (`self.HandleDestruction` (`self.PlayerInExplosionRadius`))
      (`PrimitiveComponent.SetSimulatePhysics` (`self.StaticMesh`) false)
      (`SceneComponent.SetVisibility` _staticmesh false false)
      (`PrimitiveComponent.SetCollisionEnabled` _staticmesh "NoCollision")
      (`KismetSystemLibrary.Delay` 3.0)
      (`self.K2_DestroyActor`))))

(fn `AboutToExplodeTick`
  (params (DeltaTime :type "Float (double-precision)"))
  (if (`self.bDoingCountdown`)
    (set `self.ExplosionCountdownLeft` (- (`self.ExplosionCountdownLeft`) DeltaTime))
    (`self.SetFrequency` (`KismetMathLibrary.MapRangeClamped` (`self.ExplosionCountdownLeft`) (`self.ExplosionCountdownTime`) 0.0 (`self.MinFrequency`) (`self.MaxFrequency`)))))

(fn `Apply Forces and Damage`
  (`|ExecutionSequence`
    (:`then_0`
      (bind _playerinexplosionradius (`self.PlayerInExplosionRadius`)
        (:`then`
          (bind _returnvalue (`self.K2_GetActorLocation` _playerinexplosionradius))
          (bind _distancefactor (`self.CalculateDistanceFactor` _returnvalue))
          (`PlayerCharacter.AddConstantForce` _playerinexplosionradius (* (`self.GetDirection` _returnvalue) (* (`self.ExplosionMaxFactor`) _distancefactor)))
          (`PlayerCharacter.LoseHealth` _playerinexplosionradius (* (`self.MaxDamage`) _distancefactor)))
        (:`else`)))
    (:`then_1`
      (for _array_element (`self.PhysicsActorsInRadius`)
        (bind _returnvalue_2 (`self.GetSimulatedBodyLocation` _array_element))
        (`self.AddConstantForce` _array_element (* (`self.GetDirection` _returnvalue_2) (* (`self.ExplosionMaxFactor`) (`self.CalculateDistanceFactor` _returnvalue_2))))))))

(fn `ApplyDamageToPlayer`)

(fn `BeginCountdown`
  (if (not (`self.bDoingCountdown`))
    (set `self.bDoingCountdown` true)
    (set `self.ExplosionCountdownLeft` (`self.ExplosionCountdownTime`))))

(fn `CalculateDistanceFactor`
  (params (Location :type "Vector Structure"))
  (returns (DistanceFactor :type "Float (double-precision)"))
  (locals (L_SquareDistance :type "Float (double-precision)" :default 0.0))
  (set `local.L_SquareDistance` (`KismetMathLibrary.Vector_DistanceSquared` Location (`SceneComponent.K2_GetComponentLocation` (`self.StaticMesh`))))
  (return (`KismetMathLibrary.MapRangeClamped` (`local.L_SquareDistance`) (`self.MinDistanceSquaredForFactor`) (`self.MaxDistanceSquaredForFactor`) 1.0 0.1)))

(fn `GetDirection`
  (params (Location :type "Vector Structure"))
  (returns (DirectionTowards :type "Vector Structure"))
  (locals (L_SquareDistance :type "Float (double-precision)" :default 0.0))
  (return (`KismetMathLibrary.Normal` (- Location (`SceneComponent.K2_GetComponentLocation` (`self.StaticMesh`))))))

(fn `SetFrequency`
  (params (Frequency :type "Float (double-precision)"))
  (`MeshComponent.SetScalarParameterValueOnMaterials` (`self.StaticMesh`) "Frequency" Frequency))

(fn `UserConstructionScript`
  (`parent.UserConstructionScript`))