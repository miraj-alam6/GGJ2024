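; Base interactable actor, named as not for direct use, that notifies actors when they enter or leave its proximity sphere.
; Every tick it teleports the sphere to the static mesh's world location so the detection area follows the mesh.
; Sphere overlaps send enter and exit nearby messages to the other actor, passing itself, then call empty extra functions that serve as hooks.
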(event `self.ReceiveTick`
  (params (DeltaSeconds :type "Float (single-precision)"))
  (`parent.ReceiveTick` DeltaSeconds)
  (`SceneComponent.K2_SetWorldLocation` (`self.Sphere`) (`SceneComponent.K2_GetComponentLocation` (`self.StaticMesh`)) false true))

(event `self.Sphere.OnComponentBeginOverlap`
  (params (OverlappedComponent :type "PrimitiveComponent Object Reference") (OtherActor :type "Actor Object Reference") (OtherComp :type "PrimitiveComponent Object Reference") (OtherBodyIndex :type Integer) (bFromSweep :type Boolean) (SweepResult :type "HitResult Structure (by ref)"))
  (message `/Game/Blueprints/Interface/DetectNearby.OnEnterNearby` OtherActor self)
  (`self.OnNearbyEnterExtraFunction`))

(event `self.Sphere.OnComponentEndOverlap`
  (params (OverlappedComponent :type "PrimitiveComponent Object Reference") (OtherActor :type "Actor Object Reference") (OtherComp :type "PrimitiveComponent Object Reference") (OtherBodyIndex :type Integer))
  (message `/Game/Blueprints/Interface/DetectNearby.OnExitNearby` OtherActor self)
  (`self.OnNearbyExitExtraFunction`))

(fn `OnNearbyEnterExtraFunction`)

(fn `OnNearbyExitExtraFunction`)

(fn `UserConstructionScript`
  (`parent.UserConstructionScript`))