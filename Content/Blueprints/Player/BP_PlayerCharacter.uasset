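; Player character that tracks interactable physics actors, drives the player HUD and handles death and winning.
; Enter and exit events maintain a nearby list, scanned each Tick for the closest unconsumed target by squared distance, with priority actors counting as zero, to update the interact prompt.
; Death shows a HUD message, loops an animation and spins the XZ-constrained capsule with random torque.
; Winning shows notifications, then pauses and freezes time.
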(event `self.ReceiveBeginPlay`
  (bind _returnvalue (`|CreateWidget` "/Game/UI/PlayerHud.PlayerHud_C" (`GameplayStatics.GetPlayerController` 0)))
  (set `self.PlayerHUD` _returnvalue)
  (`/Game/UI/PlayerHud.SetPlayerRef` (`self.PlayerHUD`) self)
  (`UserWidget.AddToViewport` (`self.PlayerHUD`) 0))

(event `self.ReceiveTick`
  (params (DeltaSeconds :type "Float (single-precision)"))
  (`self.ManageObjectToInteractWith`))

(event `/Game/Blueprints/Interface/DetectNearby.OnEnterNearby`
  (params (CustomPhysicsActor :type "CustomPhysicsActor Object Reference"))
  (`KismetArrayLibrary.Array_AddUnique` (`self.AllThingsNearby`) CustomPhysicsActor))

(event `/Game/Blueprints/Interface/DetectNearby.OnExitNearby`
  (params (CustomPhysicsActor :type "CustomPhysicsActor Object Reference"))
  (`KismetArrayLibrary.Array_RemoveItem` (`self.AllThingsNearby`) CustomPhysicsActor))

(event `self.Die`
  (`parent.Die`)
  (`/Game/UI/PlayerHud.ShowYouAreDead` (`self.PlayerHUD`) true)
  (`SkeletalMeshComponent.PlayAnimation` (`self.Mesh`) null true)
  (`PrimitiveComponent.SetConstraintMode` (`self.CapsuleComponent`) "XZPlane")
  (`PrimitiveComponent.AddTorqueInDegrees` (`self.CapsuleComponent`) (`KismetMathLibrary.MakeVector` 0.0 (select `bool` (`KismetMathLibrary.RandomBool`) :`false` (`KismetMathLibrary.RandomFloatInRange` 2000.0 5000.0) :`true` (`KismetMathLibrary.RandomFloatInRange` -5000.0 -2000.0))) "None" true))

(event `WinGame`
  (`self.ShowNotification` "You shut down the A.I!")
  (`/Game/UI/PlayerHud.ShowYouWin` (`self.PlayerHUD`) true)
  (`KismetSystemLibrary.Delay` 0.2)
  (`GameplayStatics.SetGamePaused` true)
  (`GameplayStatics.SetGlobalTimeDilation` 0.0))

(fn `ManageObjectToInteractWith`
  (locals (L_SmallestSquareDistance :type "Float (double-precision)" :default 900000000.0) (L_CurrentSquareDistance :type "Float (double-precision)" :default 0.0) (L_CurrentClosest :type "CustomPhysicsActor Object Reference") (L_CurrentActor :type "CustomPhysicsActor Object Reference"))
  (set `local.L_SmallestSquareDistance` 900000000.0)
  (set `self.ObjectToInteractWith` null)
  (for _array_element (`self.AllThingsNearby`)
    (set `local.L_CurrentActor` _array_element)
    (if (not (`CustomPhysicsActor.GetIsConsumed` (`local.L_CurrentActor`)))
      (if (`CustomPhysicsActor.GetPriorityForInteraction` (`local.L_CurrentActor`))
        (set `local.L_CurrentSquareDistance` 0.0)
        (else
          (set `local.L_CurrentSquareDistance` (`KismetMathLibrary.Vector_DistanceSquared` (`self.K2_GetActorLocation`) (`CustomPhysicsActor.GetSimulatedBodyLocation` (`local.L_CurrentActor`))))))
      (if (< (`local.L_CurrentSquareDistance`) (`local.L_SmallestSquareDistance`))
        (set `local.L_CurrentClosest` (`local.L_CurrentActor`))
        (set `local.L_SmallestSquareDistance` (`local.L_CurrentSquareDistance`)))))
  (bind _l_currentclosest (`local.L_CurrentClosest`)
    (:`then`
      (set `self.ObjectToInteractWith` _l_currentclosest)
      (if (`CustomPhysicsActor.GetIsConsumed` (`self.ObjectToInteractWith`))
        (`/Game/UI/PlayerHud.SetEmptyInteractText` (`self.PlayerHUD`))
        (else
          (`/Game/UI/PlayerHud.Set Interact Text` (`self.PlayerHUD`) (`self.ObjectToInteractWith`)))))
    (:`else`
      (`/Game/UI/PlayerHud.SetEmptyInteractText` (`self.PlayerHUD`)))))

(fn `ShowNotification`
  (params (NotificationText :type Text) (Duration :type "Float (double-precision)" :default 5.0))
  (`/Game/UI/PlayerHud.ShowNotification` (`self.PlayerHUD`) NotificationText Duration))

(fn `UserConstructionScript`)